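; Patrolling enemy character that damages the player on contact and dies when stomped on the head.
; Walking loops AI moves through two to four placed points with random pauses, continuing even when a move fails.
; Head overlap with the player's EnemyHit component triggers a one-time Kill: fall animation, disabled pawn/camera collision, upward player bounce, delayed destroy.
; Hit overlap applies damage to the player while the enemy is alive.
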(event OnComponentBeginOverlap(Head)
  (params (OverlappedComponent :type Primitive%20Component%20Object%20Reference) (OtherActor :type Actor%20Object%20Reference) (OtherComp :type Primitive%20Component%20Object%20Reference) (OtherBodyIndex :type Integer) (bFromSweep :type Boolean) (SweepResult :type Hit%20Result%20Structure%20%28by%20ref%29))
  (bind _asbp_third_person_character (Utilities|Casting|CastToBP_ThirdPersonCharacter OtherActor))
  (Variables|Default|SetPlayerRef _asbp_third_person_character)
  (if (== OtherComp (Variables|/Game/ThirdPerson/Blueprints/BP_ThirdPersonCharacter.BP_ThirdPersonCharacter_C|GetEnemyHit _asbp_third_person_character))
    (CallFunction|Kill)))

(event OnComponentBeginOverlap(Hit)
  (params (OverlappedComponent :type Primitive%20Component%20Object%20Reference) (OtherActor :type Actor%20Object%20Reference) (OtherComp :type Primitive%20Component%20Object%20Reference) (OtherBodyIndex :type Integer) (bFromSweep :type Boolean) (SweepResult :type Hit%20Result%20Structure%20%28by%20ref%29))
  (bind _asbp_third_person_character (Utilities|Casting|CastToBP_ThirdPersonCharacter OtherActor))
  (if (not (Variables|Default|GetDead))
    (Game|Damage|ApplyDamage _asbp_third_person_character 2e+01 0 0)))

(event Custom|Walking
  (AI|AIMoveTo self "0, 0, 0" (Variables|Default|GetMovePoint%201) 5.0 false
    (:OnSuccess
      _)
    (:OnFail
      _))
  (Utilities|FlowControl|Delay (Math|Random|RandomFloatinRange 0.5 1.0))
  (if (not (Variables|Default|GetDead))
    (AI|AIMoveTo self "0, 0, 0" (Variables|Default|GetMovePoint2) 5.0 false
      (:OnSuccess
        _)
      (:OnFail
        _))
    (Utilities|FlowControl|Delay (Math|Random|RandomFloatinRange 0.5 1.0))
    (Utilities|IsValid (Variables|Default|GetMovePoint3)
      (:Is%20Valid
        (AI|AIMoveTo self "0, 0, 0" (Variables|Default|GetMovePoint3) 5.0 false
          (:OnSuccess
            _)
          (:OnFail
            _))
        (Utilities|FlowControl|Delay (Math|Random|RandomFloatinRange 0.5 1.0))
        (Utilities|IsValid (Variables|Default|GetMovePoint4)
          (:Is%20Valid
            (AI|AIMoveTo self "0, 0, 0" (Variables|Default|GetMovePoint4) 5.0 false
              (:OnSuccess
                _)
              (:OnFail
                _))
            (Utilities|FlowControl|Delay (Math|Random|RandomFloatinRange 0.5 1.0)))
          (:Is%20Not%20Valid
            _)))
      (:Is%20Not%20Valid
        _))
    (if (not (Variables|Default|GetDead))
      (CallFunction|Walking))))

(event Custom|Kill
  (Utilities|FlowControl|DoOnce false
    (:Completed
      (Components|Animation|PlayAnimation (Variables|Character|GetMesh) "/Game/GameCharacters/Enemy/Animations/Falling_Down.Falling_Down" false)
      (Collision|SetCollisionResponsetoChannel (Variables|Collision|GetCapsuleComponent) "ECC_Pawn" "ECR_Ignore")
      (Collision|SetCollisionResponsetoChannel (Variables|Collision|GetCapsuleComponent) "ECC_Camera" "ECR_Ignore")
      (Variables|Default|SetDead true)
      (Variables|/Script/Engine.CharacterMovementComponent|SetMaxWalkSpeed (Variables|Character|GetCharacterMovement) 0.0)
      (Character|LaunchCharacter (Variables|Default|GetPlayerRef) "0.000000,0.000000,500.000000" false false)
      (Utilities|FlowControl|Delay 4.0)
      (Actor|DestroyActor))))

(event EventBeginPlay
  (CallFunction|Walking))

(fn ConstructionScript)